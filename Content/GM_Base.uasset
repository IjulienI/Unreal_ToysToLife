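; Base game mode Blueprint that starts the TTL gameplay subsystem's tag reader for physical figurines when play begins.
; BeginPlay turns off the simulator, starts the reader, assigns the figurine data table and binds handlers for tag placed and removed events.
; A placed tag that was found prints the figurine's UID and name, while tag removal does nothing.
; An unconnected switch on figurine type is left unused.
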(event Custom|OnTagPlaced
  (params (Event :type NFC%20Figurine%20Event%20Structure%20%28by%20ref%29))
  (bind (_uid _figurinedata _bwasfound) (Utilities|Struct|BreakNFCFigurineEvent Event))
  (bind (_uid_2 _name _type) (Utilities|Struct|BreakFigurineData _figurinedata))
  (if _bwasfound
    (Development|PrintString (Utilities|String|ToString(Text) (Utilities|Text|FormatText "{UID} : {Name}" _uid_2 _name)))))

(event Custom|OnTagRemoved
  (params (Event :type NFC%20Figurine%20Event%20Structure%20%28by%20ref%29)))

(event EventBeginPlay
  (bind _returnvalue (Subsystems|GetTTLGameplaySubsystem))
  (Variables|/Script/ToysToLife.TTL_GameplaySubsystem|SetbUseSimulator _returnvalue false)
  (Class|TTLGameplaySubsystem|StartReader _returnvalue)
  (Variables|/Script/ToysToLife.TTL_GameplaySubsystem|SetFigurineDataTable _returnvalue (Variables|Default|GetFigurineDatatable))
  (EventDispatchers|BindEventtoOnTagPlaced _returnvalue (EventDispatchers|CreateEvent :!event Custom|OnTagPlaced))
  (EventDispatchers|BindEventtoOnTagRemoved _returnvalue (EventDispatchers|CreateEvent :!event Custom|OnTagRemoved)))

(fn ConstructionScript)